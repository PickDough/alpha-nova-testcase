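; BP_RollySphere is a rolling-sphere pawn Blueprint that acts as the red member of a colored-pawn system.
; On BeginPlay it sets itself to Red and registers its static mesh with the ColoredPawnWorldSubsystem.
; When it hits another pawn while wearing RollySphereMaterial, it copies that material over, reports the recolor to the subsystem and marks the pawn Red.
; With any other material, it defers to the parent's hit handling.
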(event EventBeginPlay
  (|CallParentFunction)
  (bind _output_get (Variables|Default|SetPawnColor "VE_Red"))
  (Class|ColoredPawnWorldSubsystem|RegisterPawn (Subsystems|GetColoredPawnWorldSubsystem) (Variables|Default|GetStaticMesh self) _output_get))

(event Collision|EventActorBeginOverlap
  (params (OtherActor :type Actor%20Object%20Reference))
  (|CallParentFunction OtherActor) ; This node is disabled and will not be called.\nDrag off pins to build functionality.
)

(event EventTick
  (params (DeltaSeconds :type Float%20%28single-precision%29))
  (|CallParentFunction DeltaSeconds) ; This node is disabled and will not be called.\nDrag off pins to build functionality.
)

(fn ConstructionScript
  (|CallParentFunction))

(fn OnHitOtherPawn
  (params (Other :type BP%20Recolorable%20Pawn%20Object%20Reference))
  (bind _staticmesh (Variables|Default|GetStaticMesh))
  (bind _returnvalue (Rendering|Material|GetMaterial _staticmesh 0))
  (if (== _returnvalue "/Game/Components/Pawns/RollySphere/Materials/RollySphereMaterial.RollySphereMaterial")
    (Rendering|Material|SetMaterial (Variables|/Game/Components/Pawns/BP_RecolorablePawn.BP_RecolorablePawn_C|GetStaticMesh Other) 0 _returnvalue)
    (Class|ColoredPawnWorldSubsystem|OnRecolor (Subsystems|GetColoredPawnWorldSubsystem) (Variables|/Game/Components/Pawns/BP_RecolorablePawn.BP_RecolorablePawn_C|GetPawnColor Other) "VE_Red")
    (Variables|/Game/Components/Pawns/BP_RecolorablePawn.BP_RecolorablePawn_C|SetPawnColor Other "VE_Red")
    (else
      (|CallParentFunction Other))))